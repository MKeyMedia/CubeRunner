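; Game mode that handles linear level progression, restart and completion screens.
; BeginPlay sets game-only input, then finds the current level in the Levels array to store the following one, or "End" for the last.
; LevelComplete shows a completion widget and opens the next level after a timer, or shows the game-complete widget with UI-only input.
; Despite its name, EndGame reloads the current level.
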(event `self.ReceiveBeginPlay`
  (bind _returnvalue (`GameplayStatics.GetPlayerController` 0))
  (bind _levels (`self.Levels`))
  (bind _returnvalue_2 (- (`KismetArrayLibrary.Array_Length` _levels) 1))
  (`WidgetBlueprintLibrary.SetInputMode_GameOnly` _returnvalue)
  (set `PlayerController.bShowMouseCursor` false _returnvalue)
  (bind _returnvalue_3 (`GameplayStatics.GetCurrentLevelName` true))
  (for (_array_element _array_index) _levels :!label _label
    (set `self.CurentIndex` _array_index)
    (if (and (`KismetStringLibrary.EqualEqual_StrStr` _array_element _returnvalue_3) (< (`self.CurentIndex`) _returnvalue_2))
      (set `self.NextLevel` (`|GetArrayItem` (`self.Levels`) (+ (`self.CurentIndex`) 1)))
      (`self.BreakLoop`)
      (elif (== (`self.CurentIndex`) _returnvalue_2)
        (set `self.NextLevel` "End")
        (`self.BreakLoop`)))))

(event `BreakLoop`
  (goto _label :!via `Break`))

(fn `End_Game`
  (bind _returnvalue (`GameplayStatics.GetCurrentLevelName` true))
  (`GameplayStatics.OpenLevel` (`KismetStringLibrary.Conv_StringToName` _returnvalue)))

(fn `Level_Complete`
  (bind _returnvalue (`GameplayStatics.GetPlayerController` 0))
  (if (`KismetStringLibrary.EqualEqual_StrStr` (`self.NextLevel`) "End")
    (bind _returnvalue_2 (`|CreateWidget` "/Game/Blueprints/WBP_GameComplete.WBP_GameComplete_C"))
    (`UserWidget.AddToViewport` _returnvalue_2 0)
    (set `PlayerController.bShowMouseCursor` true _returnvalue)
    (`WidgetBlueprintLibrary.SetInputMode_UIOnlyEx` _returnvalue _returnvalue_2)
    (else
      (bind _returnvalue_3 (`|CreateWidget` "/Game/Blueprints/WBP_LevelComplete.WBP_LevelComplete_C"))
      (bind _output_get (set `self.WBP_LevelComplete` _returnvalue_3))
      (`UserWidget.AddToViewport` _output_get 0)
      (`KismetSystemLibrary.K2_SetTimer` null "Load_Next_Level" 2.0))))

(fn `Load_Next_Level`
  (if (not (`KismetStringLibrary.EqualEqual_StrStr` (`self.NextLevel`) "End"))
    (`GameplayStatics.OpenLevel` (`KismetStringLibrary.Conv_StringToName` (`self.NextLevel`)))))

(fn `UserConstructionScript`)