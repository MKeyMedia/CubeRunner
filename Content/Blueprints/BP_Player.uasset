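; Player-controlled runner that is pushed forward by physics impulses, steers sideways on input, and must reach the endpoint without hitting obstacles or falling.
; Tick applies mass- and delta-scaled forward force and checks fall height, while the MoveHorizontal axis adds sideways velocity-change impulses.
; Obstacle hits, falls and endpoint overlaps report to BP_GameMode.
; GameEnded halts movement after a hit or completion, but the fall check never sets it.
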(event `self.ReceiveBeginPlay`
  (bind _returnvalue (`|CreateWidget` "/Game/Blueprints/WBP_HUD.WBP_HUD_C"))
  (`UserWidget.AddToViewport` _returnvalue 0)
  (bind _asbp_game_mode (cast `/Game/Blueprints/BP_GameMode` (`GameplayStatics.GetGameMode`)))
  (set `self.BP Game Mode` _asbp_game_mode))

(event `self.ReceiveTick`
  (params (DeltaSeconds :type "Float (single-precision)"))
  (bind (_returnvalue_x _returnvalue_y _returnvalue_z) (`KismetMathLibrary.BreakVector` (`self.K2_GetActorLocation`)))
  (bind _output_get (set `self.Delta Seconds` DeltaSeconds))
  (if (not (`self.bGameEnded`))
    (`PrimitiveComponent.AddImpulse` (`self.Player`) (`KismetMathLibrary.MakeVector` (* _output_get (* (`PrimitiveComponent.GetMass` (`self.Player`)) (`self.Forward Force`)))) "None" false)
    (if (< _returnvalue_z -50.0)
      (`/Game/Blueprints/BP_GameMode.End_Game` (`self.BP Game Mode`)))))

(event `InputAxis|MoveHorizontal`
  (params (AxisValue :type "Float (single-precision)"))
  (if (not (`self.bGameEnded`))
    (`PrimitiveComponent.AddImpulse` (`self.Player`) (`KismetMathLibrary.MakeVector` 0.0 (* AxisValue (* (* (`PrimitiveComponent.GetMass` (`self.Player`)) (`self.SideWaysForce`)) (`self.Delta Seconds`)))) "None" true)))

(event `self.Player.OnComponentHit`
  (params (HitComponent :type "PrimitiveComponent Object Reference") (OtherActor :type "Actor Object Reference") (OtherComp :type "PrimitiveComponent Object Reference") (NormalImpulse :type "Vector Structure") (Hit :type "HitResult Structure (by ref)"))
  (cast `/Game/Blueprints/BP_Obstacle` OtherActor)
  (`self.GameOver`))

(event `self.Player.OnComponentBeginOverlap`
  (params (OverlappedComponent :type "PrimitiveComponent Object Reference") (OtherActor :type "Actor Object Reference") (OtherComp :type "PrimitiveComponent Object Reference") (OtherBodyIndex :type Integer) (bFromSweep :type Boolean) (SweepResult :type "HitResult Structure (by ref)"))
  (cast `/Game/Blueprints/BP_Endpoint` OtherActor)
  (set `self.bGameEnded` true)
  (`/Game/Blueprints/BP_GameMode.Level_Complete` (`self.BP Game Mode`)))

(fn `GameOver`
  (if (not (`self.bGameEnded`))
    (set `self.bGameEnded` true)
    (`/Game/Blueprints/BP_GameMode.End_Game` (`self.BP Game Mode`))))

(fn `UserConstructionScript`)